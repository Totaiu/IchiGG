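; BP_QuestionTrigger_ChildFourth is a child question trigger for the mini game that presents the fourth question when an actor overlaps it.
; The first overlap fades the camera out and, after a short delay, creates and shows the W_FourthQuestion widget with the mouse cursor enabled.
; A DoOnce gate keeps it from firing again, and the overlapping actor is not filtered.
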(event `self.ReceiveActorBeginOverlap`
  (params (OtherActor :type "Actor Object Reference"))
  (bind _returnvalue (`GameplayStatics.GetPlayerController` 0))
  (`/Engine/EditorBlueprintResources/StandardMacros.DoOnce` false
    (:`Completed`
      (`PlayerCameraManager.StartCameraFade` :`self` (`GameplayStatics.GetPlayerCameraManager` 0) :`ToAlpha` 1.0 :`Duration` 1.0)
      (`KismetSystemLibrary.Delay` 0.9)
      (bind _returnvalue_2 (`|CreateWidget` "/Game/MiniGame/W_FourthQuestion.W_FourthQuestion_C" _returnvalue))
      (bind _output_get (set `self.FWidgetRef` _returnvalue_2))
      (`UserWidget.AddToViewport` _output_get 0)
      (set `PlayerController.bShowMouseCursor` true _returnvalue))))

(fn `UserConstructionScript`
  (`parent.UserConstructionScript`))